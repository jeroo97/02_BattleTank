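; Tank pawn Blueprint that assembles a player-drivable tank and forwards input to its C++-style movement and aiming components.
; On BeginPlay it assigns turret, barrel and track meshes, gives the tracks a physical material, and initialises TankMovement and TankAiming with them.
; Axis inputs drive movement intents and rotate the azimuth gimbal and spring arm at frame-rate-independent speed, while Fire triggers TankAiming.
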(event `self.ReceiveBeginPlay`
  (bind _lefttrack (`self.LeftTrack`))
  (bind _righttrack (`self.RightTrack`))
  (`StaticMeshComponent.SetStaticMesh` (`self.TankTurret`) "/Game/Tank_2/tank_fbx_Turret.tank_fbx_Turret")
  (`StaticMeshComponent.SetStaticMesh` (`self.Barrel`) "/Game/Tank_2/tank_fbx_Barrel.tank_fbx_Barrel")
  (`StaticMeshComponent.SetStaticMesh` _lefttrack "/Game/Tank_2/tank_fbx_Track.tank_fbx_Track")
  (`PrimitiveComponent.SetPhysMaterialOverride` _lefttrack "/Game/Tank_2/Track.Track")
  (`StaticMeshComponent.SetStaticMesh` _righttrack "/Game/Tank_2/tank_fbx_Track.tank_fbx_Track")
  (`PrimitiveComponent.SetPhysMaterialOverride` _righttrack "/Game/Tank_2/Track.Track")
  (`TankMovementComponent.Initialise` (`self.TankMovement`) (`self.LeftTrack`) (`self.RightTrack`))
  (`TankAimingComponent.Initialise` (`self.TankAiming`) (`self.Barrel`) (`self.TankTurret`)))

(event `InputAxis|AimAzimuth`
  (params (AxisValue :type "Float (single-precision)"))
  ;[1 1 1] Aim Input binding
  (`SceneComponent.K2_AddLocalRotation` (`self.Azimuth gimbal`) (`KismetMathLibrary.MakeRotator` 0.0 0.0 (* AxisValue (`GameplayStatics.GetWorldDeltaSeconds`) 120.0)) false false))

(event `InputAxis|Move Forward`
  (params (AxisValue :type "Float (single-precision)"))
  ;[1 1 1] Movement Input Binding
  (`TankMovementComponent.IntendMoveForward` (`self.TankMovement`) AxisValue))

(event `InputAxis|Move Backward`
  (params (AxisValue :type "Float (single-precision)"))
  ;[1 1 1] Movement Input Binding
  (`TankMovementComponent.IntendMoveForward` (`self.TankMovement`) AxisValue))

(event `InputAxis|AimElevation`
  (params (AxisValue :type "Float (single-precision)"))
  ;[1 1 1] Aim Input binding
  (`SceneComponent.K2_AddLocalRotation` (`self.SpringArm`) (`KismetMathLibrary.MakeRotator` 0.0 (* AxisValue (`GameplayStatics.GetWorldDeltaSeconds`) 120.0)) false false))

(event `InputAxis|Turn Right`
  (params (AxisValue :type "Float (single-precision)"))
  ;[1 1 1] Movement Input Binding
  (`TankMovementComponent.IntendTurnRight` (`self.TankMovement`) AxisValue))

(event `InputAxis|Turn Left`
  (params (AxisValue :type "Float (single-precision)"))
  ;[1 1 1] Movement Input Binding
  (`TankMovementComponent.IntendTurnRight` (`self.TankMovement`) AxisValue))

(event `InputAction|Fire`
  (params (Key :type "Key Structure"))
  ;[1 1 1] Aim Input binding
  (:`Pressed`
    (`TankAimingComponent.Fire` (`self.TankAiming`))))

(fn `UserConstructionScript`)