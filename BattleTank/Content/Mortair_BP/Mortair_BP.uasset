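; Mortair_BP is a mortar unit with a dome, a barrel and a health bar widget.
; On BeginPlay it assigns both meshes, initialises the MortairAiming component with dome as turret and barrel, and sets Projectile_BP as its projectile.
; It then links the HealthBar widget back to itself through the widget's MyTank reference and registers the dome via SetTurret.
; Aiming and firing logic lie outside these graphs.
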(event `self.ReceiveBeginPlay`
  (bind _mortairdome (`self.MortairDome`))
  (bind _mortairbarrel (`self.MortairBarrel`))
  (`StaticMeshComponent.SetStaticMesh` _mortairdome "/Game/Mortair_BP/mortar_dome.mortar_dome")
  (`StaticMeshComponent.SetStaticMesh` _mortairbarrel "/Game/Mortair_BP/mortar_barrel.mortar_barrel")
  (`TankAimingComponent.Initialise` (`self.MortairAiming`) _mortairbarrel _mortairdome)
  (`TankAimingComponent.SetProjectileBP` (`self.MortairAiming`) "/Game/Projectile/Projectile_BP.Projectile_BP_C")
  (`self.InitializeHealthBarWidget`)
  (`self.SetTurret` (`self.MortairDome`)))

(fn `InitializeHealthBarWidget`
  (bind _ashealth_bar (cast `/Game/UI/HealthBar` (`WidgetComponent.GetUserWidgetObject` (`self.HealthBar`))))
  (set `/Game/UI/HealthBar.MyTank` self _ashealth_bar)
  (return))

(fn `UserConstructionScript`)